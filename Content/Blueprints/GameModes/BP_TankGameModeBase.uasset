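; Tank game mode that handles the UI at the start and end of a match.
; GameStart sets Game and UI input mode and shows a WBP_GameStart countdown seeded with StartDelay.
; GameOver shows WBP_GameOver with the win or loss result, then a short timer calls QuitGame by name to open the MainMenu level.
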(event `self.GameStart`
  (`WidgetBlueprintLibrary.SetInputMode_GameAndUIEx` (`GameplayStatics.GetPlayerController` 0) null "DoNotLock" false)
  ;[1 1 1] Countdown
  (bind _returnvalue (`|CreateWidget` "/Game/Blueprints/Widgets/WBP_GameStart.WBP_GameStart_C"))
  (set `/Game/Blueprints/Widgets/WBP_GameStart.Counter` (`self.StartDelay`) _returnvalue)
  (`UserWidget.AddToViewport` _returnvalue 0))

(event `self.GameOver`
  (params (PlayerWon :type Boolean))
  (bind _returnvalue (`|CreateWidget` "/Game/Blueprints/Widgets/WBP_GameOver.WBP_GameOver_C"))
  (set `/Game/Blueprints/Widgets/WBP_GameOver.bPlayerWon` PlayerWon _returnvalue)
  (`UserWidget.AddToViewport` _returnvalue 0)
  (`KismetSystemLibrary.K2_SetTimer` null "QuitGame" 3.0))

(fn `QuitGame`
  (`GameplayStatics.OpenLevel` "MainMenu"))

(fn `UserConstructionScript`)